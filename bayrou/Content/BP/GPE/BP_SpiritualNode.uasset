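; BP_SpiritualNode is a gameplay node actor that handles the visual teardown when the node is destroyed.
; Shortly after BeginPlay, it binds a custom event to the OnNodeDestroyed notification.
; That event removes the mesh and any valid info text actor, then activates a Niagara glitter effect.
; Timed delays let the effect play and wind down before the actor destroys itself.
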(event Custom|Custom
  (bind _ns_glitter (Variables|Default|GetNS_Glitter))
  (bind _textrenderinfo (Variables|Default|GettextRenderInfo))
  (Components|DestroyComponent (Variables|Character|GetMesh))
  (Utilities|IsValid _textrenderinfo
    (:Is%20Valid
      (Actor|DestroyActor _textrenderinfo))
    (:Is%20Not%20Valid
      _))
  (Components|Activation|Activate _ns_glitter false)
  (Utilities|FlowControl|Delay 2.0)
  (Components|Activation|Deactivate _ns_glitter)
  (Utilities|FlowControl|Delay 2.0)
  (Actor|DestroyActor))

(event EventBeginPlay
  (Utilities|FlowControl|Delay 0.1)
  (EventDispatchers|BindEventtoOnNodeDestroyed (delegate Custom|Custom)))

(event Collision|EventActorBeginOverlap
  (params (OtherActor :type Actor%20Object%20Reference)))

(event EventTick
  (params (DeltaSeconds :type Float%20%28single-precision%29)))

(fn ConstructionScript)