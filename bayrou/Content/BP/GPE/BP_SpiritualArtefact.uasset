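; BP_SpiritualArtefact is a gameplay element that can open a linked door and has a shield effect.
; On BeginPlay it activates the NSShield component and binds handlers to its OnStopNS and OnOpenDoor events, which are triggered outside this graph.
; OnOpenDoor opens DoorToOpen if valid.
; OnStopNS destroys the optional TutoText actor and removes the shield component.
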(event Custom|CustomEvent_0
  (bind _doortoopen (Variables|Default|GetdoorToOpen))
  (Utilities|IsValid _doortoopen
    (:Is%20Valid
      (Default|OpenDoor _doortoopen))))

(event Custom|CustomEvent_1
  (bind _tutotext (Variables|Default|GettutoText))
  (Utilities|IsValid _tutotext
    (:Is%20Valid
      (Actor|DestroyActor _tutotext))
    (:Is%20Not%20Valid
      _))
  (Components|DestroyComponent (Variables|Default|GetNS_Shield)))

(event EventBeginPlay
  (Components|Activation|Activate (Variables|Default|GetNS_Shield) false)
  (EventDispatchers|BindEventtoOnStopNS (delegate Custom|CustomEvent_1))
  (EventDispatchers|BindEventtoOnOpenDoor (delegate Custom|CustomEvent_0)))

(event Collision|EventActorBeginOverlap
  (params (OtherActor :type Actor%20Object%20Reference)))

(event EventTick
  (params (DeltaSeconds :type Float%20%28single-precision%29)))

(fn ConstructionScript)