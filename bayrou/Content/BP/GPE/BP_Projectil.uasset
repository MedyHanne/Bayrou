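; BP_Projectil is a projectile actor that changes the player character's health on contact.
; Tick moves it forward at constant speed with unswept SetActorLocation, and a life span set at BeginPlay removes it after a few seconds.
; Overlapping a BP_ThirdPersonCharacter passes Damage to its health component's AddLife, prints a debug string and destroys the projectile; other actors are ignored.
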(event EventBeginPlay
  (Actor|SetLifeSpan 5.0))

(event Collision|EventActorBeginOverlap
  (params (OtherActor :type Actor%20Object%20Reference))
  (bind _asbp_third_person_character (Utilities|Casting|CastToBP_ThirdPersonCharacter OtherActor))
  (Default|AddLife (Variables|/Game/ThirdPerson/Blueprints/BP_ThirdPersonCharacter.BP_ThirdPersonCharacter_C|Get3C_HealthComponent _asbp_third_person_character) (Variables|Default|GetDamage))
  (Development|PrintString "Damage")
  (Actor|DestroyActor))

(event EventTick
  (params (DeltaSeconds :type Float%20%28single-precision%29))
  (Transformation|SetActorLocation (+ (Transformation|GetActorLocation) (* (Transformation|GetActorForwardVector) (* DeltaSeconds 1e+02))) false false))

(fn ConstructionScript)