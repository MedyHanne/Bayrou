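; Spiritual artefact pickup that stays shielded until its linked nodes are destroyed, then can be recovered to open a door.
; It tracks a capped list of registered nodes; when removals empty it, the shield component is destroyed and recovery unlocks.
; Once unlocked, Tick polls player distance and the hard-coded E key.
; Recovery destroys the artefact and calls OpenDoor on its door reference.
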(event Custom|StopNS
  (Components|DestroyComponent (Variables|Default|GetNS_Shield)))

(event Custom|Open%20door
  (bind _door (Variables|Default|GetDoor))
  (Utilities|IsValid _door
    (:Is%20Valid
      (Default|OpenDoor _door))))

(event EventBeginPlay)

(event Collision|EventActorBeginOverlap
  (params (OtherActor :type Actor%20Object%20Reference)))

(event EventTick
  (params (DeltaSeconds :type Float%20%28single-precision%29))
  (CallFunction|Check))

(fn ConstructionScript)

(fn AddNode
  (params (nodeToAdd :type BP%20New%20Spiritual%20Node%20Object%20Reference))
  (bind _nodestodestroy (Variables|Default|GetnodesToDestroy))
  (Utilities|IsValid nodeToAdd
    (:Is%20Valid
      (if (not (Utilities|Array|ContainsItem _nodestodestroy nodeToAdd))
        (if (<= (Utilities|Array|Length _nodestodestroy) (Variables|Default|GetmaxCount))
          (Utilities|Array|Add (Variables|Default|GetnodesToDestroy) nodeToAdd))))))

(fn CheckRecover
  (if (== (Utilities|Array|Length (Variables|Default|GetnodesToDestroy)) 0)
    (Variables|Default|SetcanBeRecover true)
    (CallFunction|StopNS)))

(fn Reward
  (params (player :type Character%20Object%20Reference))
  (Actor|DestroyActor)
  (CallFunction|OpenDoor))

(fn DestroyNode
  (params (toDestroy :type BP%20New%20Spiritual%20Node%20Object%20Reference))
  (Utilities|IsValid toDestroy
    (:Is%20Valid
      (if (Utilities|Array|ContainsItem (Variables|Default|GetnodesToDestroy) toDestroy)
        (Utilities|Array|RemoveItem (Variables|Default|GetnodesToDestroy) toDestroy)
        (CallFunction|CheckRecover)))))

(fn Check
  (if (Variables|Default|GetcanBeRecover)
    (bind _output_get (Variables|Default|SetisPlayerInRange (<= (Math|Vector|Distance(Vector) (Transformation|GetActorLocation) (Transformation|GetActorLocation (Game|GetPlayerCharacter 0))) (Variables|Default|GetinteractionDistance))))
    (if (and (Game|Player|IsInputKeyDown (Game|GetPlayerController 0) "E") _output_get)
      (CallFunction|Reward (Game|GetPlayerCharacter 0)))))