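; BP_GrapplePoint is a grapple target that shows a proximity prompt and tells the player character when it can grapple.
; Overlapping VisibilityBox reveals a W_GrapplePrompt widget and starts a looping timer, both undone on exit.
; TrackDistance fills the prompt as the player nears TriggerSphere's edge.
; Near full, it passes itself and CanGrapple to BP_ThirdPersonCharacterRaph, using paired DoOnce gates that re-arm each other to update only on threshold crossings.
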(event OnComponentBeginOverlap(VisibilityBox)
  (params (OverlappedComponent :type Primitive%20Component%20Object%20Reference) (OtherActor :type Actor%20Object%20Reference) (OtherComp :type Primitive%20Component%20Object%20Reference) (OtherBodyIndex :type Integer) (bFromSweep :type Boolean) (SweepResult :type Hit%20Result%20Structure%20%28by%20ref%29))
  (Variables|Default|SetPlayerChar OtherActor)
  (Development|SetHiddeninGame (Variables|Default|GetW_ButtonPrompt) false false)
  (bind _returnvalue (Utilities|Time|SetTimerbyEvent (EventDispatchers|CreateEvent :!event Custom|TrackDistance) 0.1 true)))

(event OnComponentEndOverlap(VisibilityBox)
  (params (OverlappedComponent :type Primitive%20Component%20Object%20Reference) (OtherActor :type Actor%20Object%20Reference) (OtherComp :type Primitive%20Component%20Object%20Reference) (OtherBodyIndex :type Integer))
  (Development|SetHiddeninGame (Variables|Default|GetW_ButtonPrompt) true false)
  (Utilities|Time|ClearandInvalidateTimerbyHandle (stale OnComponentBeginOverlap(VisibilityBox) _returnvalue)))

(event Custom|TrackDistance
  (bind _returnvalue (Game|GetPlayerCharacter 0))
  (bind _triggersphere (Variables|Default|GetTriggerSphere))
  (bind _triggersphere_2 (Variables|Default|GetTriggerSphere))
  (bind _returnvalue_2 (Components|Sphere|GetScaledSphereRadius _triggersphere))
  (bind _returnvalue_3 (Transformation|GetActorLocation _returnvalue))
  (bind _returnvalue_4 (Transformation|GetWorldLocation _triggersphere_2))
  (bind _returnvalue_5 (- _returnvalue_4 _returnvalue_3))
  (bind _returnvalue_6 (Math|Vector|VectorLength _returnvalue_5))
  (bind _returnvalue_7 (- _returnvalue_6 _returnvalue_2))
  (bind _returnvalue_8 (Math|Float|Max(Float) _returnvalue_7 0.0))
  (bind _returnvalue_9 (/ _returnvalue_8 1e+02))
  (bind _returnvalue_10 (- _returnvalue_9 1.0))
  (bind _returnvalue_11 (Math|Float|Absolute(Float) _returnvalue_10))
  (if (< _returnvalue_10 0.0)
    (Default|SetPercent (Variables|Default|GetW_GP) _returnvalue_11)
    (if (> _returnvalue_11 0.95)
      (Utilities|FlowControl|DoOnce false
        (:Completed
          (Variables|Default|SetCanGrapple true)
          (bind _asbp_third_person_character_raph (Utilities|Casting|CastToBP_ThirdPersonCharacterRaph (Variables|Default|GetPlayerChar)))
          (Variables|/Game/ThirdPerson/Blueprints/BP_ThirdPersonCharacterRaph.BP_ThirdPersonCharacterRaph_C|SetGrapplePoint _asbp_third_person_character_raph self)
          (Variables|/Game/ThirdPerson/Blueprints/BP_ThirdPersonCharacterRaph.BP_ThirdPersonCharacterRaph_C|SetcanGrapple _asbp_third_person_character_raph (Variables|Default|GetCanGrapple))
          (CallFunction|Toggleon)))
      (else
        (Utilities|FlowControl|DoOnce true
          (:Completed
            (Variables|Default|SetCanGrapple false)
            (bind _asbp_third_person_character_raph_2 (Utilities|Casting|CastToBP_ThirdPersonCharacterRaph (Variables|Default|GetPlayerChar)))
            (Variables|/Game/ThirdPerson/Blueprints/BP_ThirdPersonCharacterRaph.BP_ThirdPersonCharacterRaph_C|SetcanGrapple _asbp_third_person_character_raph_2 (Variables|Default|GetCanGrapple))
            (CallFunction|ToggleOff)))))
    (else
      (Default|SetPercent (Variables|Default|GetW_GP) 0.0))))

(event Custom|ToggleOff
  (Utilities|FlowControl|DoOnce false) ; enters at Reset
)

(event Custom|ToggleOn
  (Utilities|FlowControl|DoOnce true) ; enters at Reset
)

(event EventBeginPlay
  (bind _returnvalue (UserInterface|CreateWidget "/Game/BP/GPE/New/GrappingV2/W_GrapplePrompt.W_GrapplePrompt_C"))
  (bind _output_get (Variables|Default|SetW_GP _returnvalue))
  (UserInterface|SetWidget (Variables|Default|GetW_ButtonPrompt) _output_get))

(fn ConstructionScript)