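; BP_BouncingZone is a trigger zone that bounces Characters forward and upward when they enter its box.
; On overlap, it flattens the character's forward vector, adds an up vector scaled by vertical strength, then overwrites the movement component's velocity directly.
; The whole sum is multiplied by forward strength and divided by a fixed constant, so forward strength also scales the vertical bounce.
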(event OnComponentBeginOverlap(Box)
  (params (OverlappedComponent :type Primitive%20Component%20Object%20Reference) (OtherActor :type Actor%20Object%20Reference) (OtherComp :type Primitive%20Component%20Object%20Reference) (OtherBodyIndex :type Integer) (bFromSweep :type Boolean) (SweepResult :type Hit%20Result%20Structure%20%28by%20ref%29))
  (bind _ascharacter (Utilities|Casting|CastToCharacter OtherActor))
  (bind _output_get (Variables|Default|SetforwardDir (Math|Vector|MakeVector (.x (Transformation|GetActorForwardVector _ascharacter)) (.y (Transformation|GetActorForwardVector _ascharacter)) 0.0)))
  (Variables|/Script/Engine.MovementComponent|SetVelocity (Variables|/Script/Engine.Character|GetCharacterMovement _ascharacter) (/ (* (+ _output_get (* (Math|Vector|VectorUp) (Variables|Default|GetVerticalBounceStrength))) (Variables|Default|GetForwardBounceStrength)) 2e+03)))

(event EventBeginPlay)

(event Collision|EventActorBeginOverlap
  (params (OtherActor :type Actor%20Object%20Reference)))

(event EventTick
  (params (DeltaSeconds :type Float%20%28single-precision%29)))

(fn ConstructionScript)