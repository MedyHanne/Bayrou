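; BP_NewConfusiusRetreat is a proximity-based interactable that the player triggers with the E key.
; Every tick, Check compares the distance to the player character against InteractionDistance, activating the glitter effect in range and deactivating it outside.
; While in range, it polls the E key directly on the player controller and calls Reward, which currently only destroys the actor.
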(event EventBeginPlay)

(event EventTick
  (params (DeltaSeconds :type Float%20%28single-precision%29))
  (CallFunction|Check))

(fn ConstructionScript)

(fn Reward
  (params (Player :type Character%20Object%20Reference))
  (Actor|DestroyActor))

(fn Check
  (bind _ns_glitter1 (Variables|Default|GetNS_Glitter1))
  (bind _output_get (Variables|Default|SetisPlayerInRange (<= (Math|Vector|Distance(Vector) (Transformation|GetActorLocation) (Transformation|GetActorLocation (Game|GetPlayerCharacter 0))) (Variables|Default|GetinteractionDistance))))
  (if _output_get
    (Components|Activation|Activate _ns_glitter1 false)
    (if (Game|Player|IsInputKeyDown (Game|GetPlayerController 0) "E")
      (CallFunction|Reward (Game|GetPlayerCharacter 0)))
    (else
      (Components|Activation|Deactivate _ns_glitter1))))