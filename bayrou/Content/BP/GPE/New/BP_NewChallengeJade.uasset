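; Timed race challenge that starts when the player dashes into its mesh and rewards finishing in time with extra max health.
; Starting reveals platforms and checkpoints, activates the EndZone, shows the HUD timer and later makes the mesh block pawns.
; Tick advances the timer and fails the race at the limit, resetting it for retry.
; The EndZone's end event triggers success, which heals, hides the course and briefly shows a win popup.
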(event OnComponentBeginOverlap(StaticMesh)
  (params (OverlappedComponent :type Primitive%20Component%20Object%20Reference) (OtherActor :type Actor%20Object%20Reference) (OtherComp :type Primitive%20Component%20Object%20Reference) (OtherBodyIndex :type Integer) (bFromSweep :type Boolean) (SweepResult :type Hit%20Result%20Structure%20%28by%20ref%29))
  (bind _jadechallengewidget (Variables|Default|GetjadeChallengeWidget))
  (bind _allcheckpoints (Variables|Default|GetallCheckPoints))
  (Development|PrintString (Utilities|GetDisplayName OtherActor))
  (if (not (Math|Boolean|ORBoolean (Variables|Default|GetraceStarted) (Variables|Default|GetraceCompleted) (Variables|Default|GetisPlayerDashing)))
    (if (Utilities|Array|IsNotEmpty _allcheckpoints)
      (for _array_element _allcheckpoints
        (Rendering|SetVisibility (Variables|/Game/BP/GPE/New/BP_JadeCheckPoint.BP_JadeCheckPoint_C|GetStaticMesh _array_element) true false)))
    (Utilities|Casting|CastToBP_ThirdPersonCharacter OtherActor)
    (Variables|Default|SetraceStarted true)
    (bind _output_get (Variables|Default|SettimeLimitString (Utilities|String|ToString(Float) (Variables|Default|GettimeLimit))))
    (Class|JadeChallengeWidget|SetTimeLimitText _jadechallengewidget _output_get)
    (Widget|SetVisibility _jadechallengewidget "Visible")
    (Variables|Default|SetcurrentTime 0.0)
    (CallFunction|SetMaterial (Variables|Default|GetonGoingMat))
    (Variables|/Game/BP/GPE/New/BP_NewEndZone.BP_NewEndZone_C|SetisActive (Variables|Default|GetendZone) true)
    (for _array_element_2 (Variables|Default|GetallPlatforms)
      (Rendering|SetActorHiddenInGame _array_element_2 false))
    (Utilities|FlowControl|Delay 1.0)
    (Collision|SetCollisionResponsetoChannel (Variables|Default|GetStaticMesh) "ECC_Pawn" "ECR_Block")))

(event Custom|ReachEnd
  (params (overlappingActor :type Actor%20Object%20Reference))
  (CallFunction|OnPlayerReachEnd overlappingActor))

(event Custom|Delay4sec
  (Utilities|FlowControl|Delay 4.0)
  (Widget|SetVisibility (Variables|Default|GetwinPopupWidget) "Hidden"))

(event EventBeginPlay
  (bind _allcheckpoints (Variables|Default|GetallCheckPoints))
  (for _array_element (Variables|Default|GetallPlatforms)
    (Rendering|SetActorHiddenInGame _array_element true))
  (EventDispatchers|BindEventtoOnEndZoneReachEnd (Variables|Default|GetendZone) (delegate Custom|ReachEnd))
  (Utilities|FlowControl|Delay 0.2)
  (bind _asbp_player_hud (Utilities|Casting|CastToBP_Player_HUD (HUD|GetHUD (Game|GetPlayerController 0))))
  (Variables|Default|SetjadeChallengeWidget (Variables|/Script/bayrou.MainWidget|GetjadeChallengeWidget (Variables|/Script/bayrou.Player_HUD|GetmainWidget _asbp_player_hud)))
  (Variables|Default|SetwinPopupWidget (Variables|/Script/bayrou.MainWidget|GetwinPopupWidget (Variables|/Script/bayrou.Player_HUD|GetmainWidget _asbp_player_hud)))
  (if (Utilities|Array|IsNotEmpty _allcheckpoints)
    (for _array_element_2 _allcheckpoints
      (Rendering|SetVisibility (Variables|/Game/BP/GPE/New/BP_JadeCheckPoint.BP_JadeCheckPoint_C|GetStaticMesh _array_element_2) false false))))

(event Collision|EventActorBeginOverlap
  (params (OtherActor :type Actor%20Object%20Reference)))

(event EventTick
  (params (DeltaSeconds :type Float%20%28single-precision%29))
  (bind _asbp_third_person_character (Utilities|Casting|CastToBP_ThirdPersonCharacter (Game|Player|GetPlayerPawn 0)))
  (Variables|Default|SetisPlayerDashing (Variables|/Game/ThirdPerson/Blueprints/BP_ThirdPersonCharacter.BP_ThirdPersonCharacter_C|GetisNotInDash _asbp_third_person_character))
  (if (Variables|Default|GetraceStarted)
    (CallFunction|UpdateTime DeltaSeconds)))

(fn ConstructionScript)

(fn SetMaterial
  (params (newMat :type Material%20Object%20Reference))
  (Rendering|Material|SetMaterial (Variables|Default|GetStaticMesh) 0 newMat))

(fn UpdateTime
  (params (deltaTime :type Float%20%28double-precision%29))
  (bind _output_get (Variables|Default|SetcurrentTime (+ deltaTime (Variables|Default|GetcurrentTime))))
  (bind _output_get_2 (Variables|Default|SettimeString (Utilities|String|ToString(Float) _output_get)))
  (Class|JadeChallengeWidget|SetCurrentTimetText (Variables|Default|GetjadeChallengeWidget) _output_get_2)
  (if (>= (Variables|Default|GetcurrentTime) (Variables|Default|GettimeLimit))
    (Variables|Default|SetraceStarted false)
    (CallFunction|ChallenegeFailed)))

(fn ChallengeSucceeded
  (params (Player :type Actor%20Object%20Reference))
  (bind _allcheckpoints (Variables|Default|GetallCheckPoints))
  (bind _asbp_third_person_character (Utilities|Casting|CastToBP_ThirdPersonCharacter Player))
  (Development|PrintString "END" true true "(R=1.000000,G=0.051854,B=0.071750,A=1.000000)" 5.0)
  (Default|AddMaxLife (Variables|/Game/ThirdPerson/Blueprints/BP_ThirdPersonCharacter.BP_ThirdPersonCharacter_C|Get3C_HealthComponent _asbp_third_person_character) 1.0)
  (Default|AddLife (Variables|/Game/ThirdPerson/Blueprints/BP_ThirdPersonCharacter.BP_ThirdPersonCharacter_C|Get3C_HealthComponent _asbp_third_person_character) (Variables|/Game/BP/Component/3C_HealthComponent.3C_HealthComponent_C|GetmaxLife (Variables|/Game/ThirdPerson/Blueprints/BP_ThirdPersonCharacter.BP_ThirdPersonCharacter_C|Get3C_HealthComponent _asbp_third_person_character)))
  (Variables|Default|SetraceCompleted true)
  (Rendering|Material|SetMaterial (Variables|Default|GetStaticMesh) 0 (Variables|Default|GetwinMat))
  (for _array_element (Variables|Default|GetallPlatforms)
    (Rendering|SetActorHiddenInGame _array_element true))
  (if (Utilities|Array|IsNotEmpty _allcheckpoints)
    (for _array_element_2 _allcheckpoints
      (Rendering|SetVisibility (Variables|/Game/BP/GPE/New/BP_JadeCheckPoint.BP_JadeCheckPoint_C|GetStaticMesh _array_element_2) false false)))
  (Widget|SetVisibility (Variables|Default|GetjadeChallengeWidget) "Hidden")
  (Widget|SetVisibility (Variables|Default|GetwinPopupWidget) "Visible")
  (CallFunction|Delay4sec))

(fn ChallenegeFailed
  (bind _allcheckpoints (Variables|Default|GetallCheckPoints))
  (Variables|Default|SetraceCompleted false)
  (CallFunction|SetMaterial (Variables|Default|GetlooseMat))
  (Variables|/Game/BP/GPE/New/BP_NewEndZone.BP_NewEndZone_C|SetisActive (Variables|Default|GetendZone) false)
  (for _array_element (Variables|Default|GetallPlatforms)
    (Rendering|SetActorHiddenInGame _array_element true))
  (Collision|SetCollisionResponsetoChannel (Variables|Default|GetStaticMesh) "ECC_Pawn" "ECR_Overlap")
  (Widget|SetVisibility (Variables|Default|GetjadeChallengeWidget) "Hidden")
  (if (Utilities|Array|IsNotEmpty _allcheckpoints)
    (for _array_element_2 _allcheckpoints
      (Rendering|SetVisibility (Variables|/Game/BP/GPE/New/BP_JadeCheckPoint.BP_JadeCheckPoint_C|GetStaticMesh _array_element_2) false false))))

(fn OnPlayerReachEnd
  (params (overlappedActor :type Actor%20Object%20Reference))
  (Development|PrintString "Hello")
  (if (Variables|Default|GetraceStarted)
    (Variables|Default|SetraceStarted false)
    (if (< (Variables|Default|GetcurrentTime) (Variables|Default|GettimeLimit))
      (CallFunction|ChallengeSucceeded overlappedActor)
      (Variables|/Game/BP/GPE/New/BP_NewEndZone.BP_NewEndZone_C|SetisActive (Variables|Default|GetendZone) false))))