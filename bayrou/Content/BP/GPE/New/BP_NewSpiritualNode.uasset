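; Spiritual node actor that registers with an artefact and is destroyed when the player dashes into it.
; A dashing character's overlap notifies the artefact, hides the mesh, stops FoliagePlaced, activates glitter, then destroys the actor after a short delay.
; When CanTeleport is set, Tick alternates the node between its start position and TpLocation on a timer.
; The artefact reference is assigned through a setter, and non-dash overlaps only print debug text.
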(event OnComponentBeginOverlap(StaticMesh)
  (params (OverlappedComponent :type Primitive%20Component%20Object%20Reference) (OtherActor :type Actor%20Object%20Reference) (OtherComp :type Primitive%20Component%20Object%20Reference) (OtherBodyIndex :type Integer) (bFromSweep :type Boolean) (SweepResult :type Hit%20Result%20Structure%20%28by%20ref%29))
  (Utilities|IsValid (Variables|Default|GetartefactRef)
    (:Is%20Valid
      (bind _asbp_third_person_character (Utilities|Casting|CastToBP_ThirdPersonCharacter OtherActor))
      (Development|PrintString "Hello")
      (if (Variables|/Game/ThirdPerson/Blueprints/BP_ThirdPersonCharacter.BP_ThirdPersonCharacter_C|GetisNotInDash _asbp_third_person_character)
        (Development|PrintString "Hello")
        (else
          (Default|DestroyNode (Variables|Default|GetartefactRef) self)
          (Rendering|SetVisibility (Variables|Default|GetStaticMesh) false false)
          (Audio|Components|Audio|Stop (Variables|Default|GetFoliage_Placed))
          (Components|Activation|Activate (Variables|Default|GetNS_Glitter) false)
          (Utilities|FlowControl|Delay 2.0)
          (Actor|DestroyActor))))))

(event EventBeginPlay
  (Utilities|IsValid (Variables|Default|GetartefactRef)
    (:Is%20Valid
      (Default|AddNode (Variables|Default|GetartefactRef) self)
      (Variables|Default|SetstartPosition (Transformation|GetActorLocation)))))

(event EventTick
  (params (DeltaSeconds :type Float%20%28single-precision%29))
  (if (Variables|Default|GetcanTeleport)
    (bind _output_get (Variables|Default|SetcurrentTime (+ DeltaSeconds (Variables|Default|GetcurrentTime))))
    (if (>= _output_get (Variables|Default|GettimeBeforeTP))
      (Transformation|SetActorLocation (Math|Vector|SelectVector (Variables|Default|GettpLocation) (Variables|Default|GetstartPosition) (Utilities|Operators|EqualEqual (Transformation|GetActorLocation) (Variables|Default|GetstartPosition) 0.0)) false false)
      (Variables|Default|SetcurrentTime 0.0))))

(fn ConstructionScript)

(fn SetSpiritualArtefact
  (params (artefact :type BP%20New%20Spiritual%20Artefact%20Object%20Reference))
  (Variables|Default|SetartefactRef artefact))