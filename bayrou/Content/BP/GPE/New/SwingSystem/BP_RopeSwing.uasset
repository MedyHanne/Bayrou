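; Rope swing actor that the player can grab, swing, climb and jump from, with input enabled on entering its box.
; Holding Space attaches the character to the cable end at its current height; releasing detaches, launches it forward and up, and disables input.
; ZQSD set directional cable forces to swing.
; Holding E/A climbs up/down through delay loops, bounded by two reference components positioned by the construction script.
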(event OnComponentBeginOverlap(Box)
  (params (OverlappedComponent :type Primitive%20Component%20Object%20Reference) (OtherActor :type Actor%20Object%20Reference) (OtherComp :type Primitive%20Component%20Object%20Reference) (OtherBodyIndex :type Integer) (bFromSweep :type Boolean) (SweepResult :type Hit%20Result%20Structure%20%28by%20ref%29))
  ;[1 1 1] Enable Input of this BP
  (Input|EnableInput self (Game|GetPlayerController 0)))

(event Input|KeyboardEvents|SpaceBar
  (params (Key :type Key%20Structure :default "None"))
  (bind _returnvalue (Game|GetPlayerCharacter 0))
  (bind _returnvalue_2 (Game|GetPlayerCharacter 0))
  (bind _returnvalue_3 (Transformation|GetActorLocation _returnvalue_2))
  ;[1 1 1] Get On/Off rope
  (:Pressed
    (Variables|Default|SetPlayerHeight (.z (Transformation|GetActorLocation _returnvalue_2)))
    (Transformation|AttachActorToActor _returnvalue_2 (Variables|Default|GetCableRef) "CableEnd" "SnapToTarget" "KeepWorld" "KeepWorld" true)
    (Transformation|SetActorLocation _returnvalue_2 (Math|Vector|MakeVector (.x _returnvalue_3) (.y _returnvalue_3) (Variables|Default|GetPlayerHeight)) false false)
    (Pawn|Components|CharacterMovement|SetMovementMode (Variables|/Script/Engine.Character|GetCharacterMovement _returnvalue_2) "MOVE_None" 0))
  (:Released
    (Transformation|DetachFromActor _returnvalue_2 "KeepWorld" "KeepWorld" "KeepWorld")
    (Pawn|Components|CharacterMovement|SetMovementMode (Variables|/Script/Engine.Character|GetCharacterMovement _returnvalue_2) "MOVE_Falling" 0)
    (Character|LaunchCharacter _returnvalue_2 (+ (* (Transformation|GetActorForwardVector _returnvalue) 1.2e+03) (* (Transformation|GetActorUpVector _returnvalue) 2e+02)) false false)
    (Input|DisableInput (Game|GetPlayerController 0))))

(event Input|KeyboardEvents|E
  (params (Key :type Key%20Structure :default "None"))
  ;[1 1 1] Climb up / down
  (:Pressed
    (Variables|Default|SetEHeld? true)
    (if (>= (.z (Transformation|GetWorldLocation (Variables|Default|GetTopClimbRef))) (.z (Transformation|GetActorLocation (Game|GetPlayerCharacter 0)))) :!label _label
      (Transformation|AddActorWorldOffset (Game|GetPlayerCharacter 0) "0.000000,0.000000,1.000000")
      (Utilities|FlowControl|Delay 0.01)
      (if (Variables|Default|GetEHeld?)
        (goto _label))))
  (:Released
    (Variables|Default|SetEHeld? false)))

(event Input|KeyboardEvents|A
  (params (Key :type Key%20Structure :default "None"))
  ;[1 1 1] Climb up / down
  (:Pressed
    (Variables|Default|SetAHeld? true)
    (if (<= (.z (Transformation|GetWorldLocation (Variables|Default|GetBottomClimbRef))) (.z (Transformation|GetActorLocation (Game|GetPlayerCharacter 0)))) :!label _label
      (Transformation|AddActorWorldOffset (Game|GetPlayerCharacter 0) "0.000000,0.000000,-1.000000")
      (Utilities|FlowControl|Delay 0.01)
      (if (Variables|Default|GetAHeld?)
        (goto _label))))
  (:Released
    (Variables|Default|SetAHeld? false)))

(event Input|KeyboardEvents|Z
  (params (Key :type Key%20Structure :default "None"))
  ;[1 1 1] Swing Rope
  (:Pressed
    (Variables|/Script/CableComponent.CableComponent|SetCableForce (Variables|/Script/CableComponent.CableActor|GetCableComponent (Variables|Default|GetCableRef)) "100.000000,0.000000,0.000000")))

(event Input|KeyboardEvents|S
  (params (Key :type Key%20Structure :default "None"))
  ;[1 1 1] Swing Rope
  (:Pressed
    (Variables|/Script/CableComponent.CableComponent|SetCableForce (Variables|/Script/CableComponent.CableActor|GetCableComponent (Variables|Default|GetCableRef)) "-100.000000,0.000000,0.000000")))

(event Input|KeyboardEvents|Q
  (params (Key :type Key%20Structure :default "None"))
  ;[1 1 1] Swing Rope
  (:Pressed
    (Variables|/Script/CableComponent.CableComponent|SetCableForce (Variables|/Script/CableComponent.CableActor|GetCableComponent (Variables|Default|GetCableRef)) "0.000000,-100.000000,0.000000")))

(event Input|KeyboardEvents|D
  (params (Key :type Key%20Structure :default "None"))
  ;[1 1 1] Swing Rope
  (:Pressed
    (Variables|/Script/CableComponent.CableComponent|SetCableForce (Variables|/Script/CableComponent.CableActor|GetCableComponent (Variables|Default|GetCableRef)) "0.000000,100.000000,0.000000")))

(fn ConstructionScript
  (bind _topclimbref (Variables|Default|GetTopClimbRef))
  (bind _bottomclimbref (Variables|Default|GetBottomClimbRef))
  (bind _relativelocation (Variables|/Script/Engine.SceneComponent|GetRelativeLocation _topclimbref))
  (bind _relativelocation_2 (Variables|/Script/Engine.SceneComponent|GetRelativeLocation _bottomclimbref))
  (Transformation|SetRelativeLocation _topclimbref (Math|Vector|MakeVector (Variables|Default|GetTopClimbLimit) (.y _relativelocation) (.z _relativelocation)) false false)
  (Transformation|SetRelativeLocation _bottomclimbref (Math|Vector|MakeVector (Variables|Default|GetBottomClimbLimit) (.y _relativelocation_2) (.z _relativelocation_2)) false false))