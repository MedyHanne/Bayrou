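; BP_ResetJade is a trigger actor that lets a Character fail and reset a linked race challenge.
; Every Tick, it shows its mesh and text only while the referenced Chalenge is started or completed.
; A Character overlap in that state calls ChallenegeFailed, clears both race flags, then unchecks every checkpoint and resets its mesh material.
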(event EventBeginPlay)

(event Collision|EventActorBeginOverlap
  (params (OtherActor :type Actor%20Object%20Reference))
  (bind _chalenge (Variables|Default|Getchalenge))
  (bind _chalenge_2 (Variables|Default|Getchalenge))
  (bind _allcheckpoints (Variables|/Game/BP/GPE/New/BP_NewChallengeJade.BP_NewChallengeJade_C|GetallCheckPoints _chalenge))
  (Utilities|Casting|CastToCharacter OtherActor)
  (Utilities|IsValid _chalenge_2
    (:Is%20Valid
      (if (or (Variables|/Game/BP/GPE/New/BP_NewChallengeJade.BP_NewChallengeJade_C|GetraceStarted _chalenge_2) (Variables|/Game/BP/GPE/New/BP_NewChallengeJade.BP_NewChallengeJade_C|GetraceCompleted _chalenge_2))
        (Default|ChallenegeFailed _chalenge)
        (Variables|/Game/BP/GPE/New/BP_NewChallengeJade.BP_NewChallengeJade_C|SetraceStarted _chalenge false)
        (Variables|/Game/BP/GPE/New/BP_NewChallengeJade.BP_NewChallengeJade_C|SetraceCompleted _chalenge false)
        (if (Utilities|Array|IsNotEmpty _allcheckpoints)
          (for _array_element _allcheckpoints
            (Variables|/Game/BP/GPE/New/BP_JadeCheckPoint.BP_JadeCheckPoint_C|SetisCheck _array_element false)
            (Rendering|Material|SetMaterial (Variables|/Game/BP/GPE/New/BP_JadeCheckPoint.BP_JadeCheckPoint_C|GetStaticMesh _array_element) 0 "/Engine/EngineDebugMaterials/ShadedLevelColorationLitMaterial.ShadedLevelColorationLitMaterial")))))))

(event EventTick
  (params (DeltaSeconds :type Float%20%28single-precision%29))
  (bind _staticmesh (Variables|Default|GetStaticMesh))
  (bind _textrender (Variables|Default|GetTextRender))
  (bind _chalenge (Variables|Default|Getchalenge))
  (Utilities|IsValid _chalenge
    (:Is%20Valid
      (if (or (Variables|/Game/BP/GPE/New/BP_NewChallengeJade.BP_NewChallengeJade_C|GetraceStarted _chalenge) (Variables|/Game/BP/GPE/New/BP_NewChallengeJade.BP_NewChallengeJade_C|GetraceCompleted _chalenge))
        (Development|SetHiddeninGame _staticmesh false false)
        (Rendering|SetVisibility _textrender true false)
        (else
          (Development|SetHiddeninGame _staticmesh true false)
          (Rendering|SetVisibility _textrender false false))))))

(fn ConstructionScript)