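; BP_NewEndZone is the end zone of a race challenge, completed by dashing into it.
; Tick shows or hides the mesh, spotlight and target arrow from IsActive, and toggles mesh and spotlight to blink once the Challenge's remaining time falls below a threshold.
; Overlapping the mesh while active calls OnEndZoneReachEnd only if BP_NicolasThirdPersonCharacter is dashing, and leaves IsActive true.
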(event OnComponentBeginOverlap(StaticMesh)
  (params (OverlappedComponent :type Primitive%20Component%20Object%20Reference) (OtherActor :type Actor%20Object%20Reference) (OtherComp :type Primitive%20Component%20Object%20Reference) (OtherBodyIndex :type Integer) (bFromSweep :type Boolean) (SweepResult :type Hit%20Result%20Structure%20%28by%20ref%29))
  (if (Variables|Default|GetisActive)
    (bind _asbp_nicolas_third_person_character (Utilities|Casting|CastToBP_NicolasThirdPersonCharacter OtherActor))
    (if (and (Utilities|IsValid _asbp_nicolas_third_person_character) (Variables|/Game/ThirdPerson/Blueprints/BP_NicolasThirdPersonCharacter.BP_NicolasThirdPersonCharacter_C|GetisDashing _asbp_nicolas_third_person_character))
      (Variables|Default|SetisActive true)
      (Default|CallOnEndZoneReachEnd))))

(event Collision|EventActorBeginOverlap
  (params (OtherActor :type Actor%20Object%20Reference)))

(event EventTick
  (params (DeltaSeconds :type Float%20%28single-precision%29))
  (bind _staticmesh (Variables|Default|GetStaticMesh))
  (bind _targetarrow (Variables|Default|GettargetArrow))
  (bind _spotlight (Variables|Default|GetSpotLight))
  (bind _challenge (Variables|Default|Getchallenge))
  (bind _challenge_2 (Variables|Default|Getchallenge))
  (if (Variables|Default|GetisActive)
    (Rendering|SetVisibility _staticmesh true false)
    (Rendering|SetActorHiddenInGame _targetarrow false)
    (Rendering|SetVisibility _spotlight true false)
    (else
      (Rendering|SetVisibility _staticmesh false false)
      (Rendering|SetActorHiddenInGame _targetarrow true)
      (Rendering|SetVisibility _spotlight false false)))
  (if (Math|Boolean|ANDBoolean (Utilities|IsValid _challenge) (Variables|Default|GetisActive) (Variables|/Game/BP/GPE/New/BP_NewChallengeJade.BP_NewChallengeJade_C|GetraceStarted _challenge))
    (bind _output_get (Variables|Default|SettimeLeft (- (Variables|/Game/BP/GPE/New/BP_NewChallengeJade.BP_NewChallengeJade_C|GettimeLimit _challenge_2) (Variables|/Game/BP/GPE/New/BP_NewChallengeJade.BP_NewChallengeJade_C|GetcurrentTime _challenge_2))))
    (if (<= _output_get (Variables|Default|GetblinkStartTime))
      (bind _output_get_2 (Variables|Default|SetblinkTimer (+ (Variables|Default|GetblinkTimer) DeltaSeconds)))
      (if (<= _output_get_2 0.5)
        (Variables|Default|SetblinkTimer 0.0)
        (Variables|Default|SetblinkState (not (Variables|Default|GetblinkState)))
        (Rendering|SetVisibility (Variables|Default|GetSpotLight) (Variables|Default|GetblinkState) false)
        (Rendering|SetVisibility (Variables|Default|GetStaticMesh) (Variables|Default|GetblinkState) false))
      (else
        (Rendering|SetVisibility (Variables|Default|GetSpotLight) true false)))))

(fn ConstructionScript)