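; AI path-following component that moves its owning actor along a BP_SplineIA spline, with a function to respawn that spline at the owner's transform.
; Each Tick advances a looping distance by direction and speed, or run-away speed under Fear, then places the owner facing slightly ahead.
; Speed comes from distance ranges in ParcoursStats.
; A debug line draws every Tick; the color-coded DrawParkour visualization is unwired.
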(event EventBeginPlay)

(event EventTick
  (params (DeltaSeconds :type Float%20%28single-precision%29))
  (bind _returnvalue (Components|GetOwner))
  (bind _distancealongspline (Variables|Default|GetDistanceAlongSpline))
  (bind _spline (Variables|Default|GetSpline))
  (bind _spline_2 (Variables|/Game/BP/IA/BP_SplineIA.BP_SplineIA_C|GetSpline _spline))
  (bind _returnvalue_2 (Spline|GetLocationatDistanceAlongSpline _spline_2 _distancealongspline "World"))
  (CallFunction|UpdatePosition DeltaSeconds)
  (Transformation|SetActorLocation _returnvalue _returnvalue_2 false false)
  (Transformation|SetActorRotation _returnvalue (Math|Rotator|FindLookatRotation _returnvalue_2 (Spline|GetLocationatDistanceAlongSpline _spline_2 (+ _distancealongspline 1.0) "World")))
  (CallFunction|UpdateSpeed)
  (Rendering|Debug|DrawDebugLine _returnvalue_2 (+ _returnvalue_2 (* (Transformation|GetActorForwardVector _returnvalue) "100.000000,100.000000,100.000000")) "(R=1.000000,G=0.000000,B=0.059079,A=1.000000)" 1.0 0.0))

(fn GenerateSpline
  (Utilities|IsValid (Variables|Default|GetSpline)
    (:Is%20Valid
      (Actor|DestroyActor (Variables|Default|GetSpline)))
    (:Is%20Not%20Valid
      _))
  (bind _returnvalue (Game|SpawnActorfromClass "/Game/BP/IA/BP_SplineIA.BP_SplineIA_C" (Transformation|GetActorTransform (Components|GetOwner)) "AlwaysSpawn" "MultiplyWithRoot" 0 0))
  (Variables|Default|SetSpline _returnvalue))

(fn UpdatePosition
  (params (DeltaTime :type Float%20%28double-precision%29))
  (bind _spline (Variables|Default|GetSpline))
  (bind _spline_2 (Variables|/Game/BP/IA/BP_SplineIA.BP_SplineIA_C|GetSpline _spline))
  (bind _returnvalue (Spline|GetSplineLength _spline_2))
  (if (Variables|Default|GetFear)
    (LocalVariables|Setprogession (+ (* DeltaTime (Variables|Default|GetRun%20Away%20Speed) (Variables|Default|GetDirection)) (Variables|Default|GetDistanceAlongSpline)))
    (else
      (bind _output_get (LocalVariables|Setprogession (+ (* DeltaTime (Variables|Default|GetSpeed) (Variables|Default|GetDirection)) (Variables|Default|GetDistanceAlongSpline))))))
  (if (or (> (Math|Float|Absolute(Float) _output_get) _returnvalue) (< _output_get 0.0))
    (if (< (Variables|Default|GetDirection) 0.0)
      (Variables|Default|SetDistanceAlongSpline (+ (LocalVariables|Getprogession) _returnvalue))
      (else
        (Variables|Default|SetDistanceAlongSpline (- (LocalVariables|Getprogession) _returnvalue))))
    (else
      (Variables|Default|SetDistanceAlongSpline (LocalVariables|Getprogession)))))

(fn DrawParkour
  (bind _spline (Variables|Default|GetSpline))
  (bind _spline_2 (Variables|/Game/BP/IA/BP_SplineIA.BP_SplineIA_C|GetSpline _spline))
  (Rendering|Debug|DrawDebugBox (Spline|GetLocationatDistanceAlongSpline _spline_2 0.0 "World") "20.000000,20.000000,20.000000" "(R=0.000000,G=0.000000,B=0.000000,A=1.000000)" "0, 0, 0" 1e+01 0.0)
  (for _index (range 0 (Math|Float|Truncate (Spline|GetSplineLength _spline_2)))
    (LocalVariables|SetcolorChange false)
    (for _array_element (Variables|/Game/BP/IA/Component/ArrayParcourParameters.ArrayParcourParameters_C|GetParcoursStats (Variables|Default|GetArrayParcourStat))
      (if (and (> (Math|Conversions|ToFloat(Integer) _index) (.start _array_element)) (< (Math|Conversions|ToFloat(Integer) _index) (.end _array_element)))
        (LocalVariables|SetColorDebug (.debugcolor _array_element))
        (LocalVariables|SetcolorChange true)))
    (if (not (LocalVariables|GetcolorChange))
      (LocalVariables|SetColorDebug (Math|Conversions|ToColor(LinearColor) (Class|KismetMathLibrary|LinearColorYellow))))
    (Rendering|Debug|DrawDebugSphere (Spline|GetLocationatDistanceAlongSpline _spline_2 (Math|Conversions|ToFloat(Integer) _index) "World") 1e+01 12 (Math|Conversions|ToLinearColor(Color) (LocalVariables|GetColorDebug)) 1e+01)))

(fn UpdateSpeed
  (bind _distancealongspline (Variables|Default|GetDistanceAlongSpline))
  (for _array_element (Variables|/Game/BP/IA/Component/ArrayParcourParameters.ArrayParcourParameters_C|GetParcoursStats (Variables|Default|GetArrayParcourStat))
    (if (and (> _distancealongspline (.start _array_element)) (< _distancealongspline (.end _array_element)))
      (Variables|Default|SetSpeed (.speed _array_element)))))